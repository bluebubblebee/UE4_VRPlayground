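; BP_PaintBrushPurple is a VR paint brush pickup that detects when it is aimed at a nearby canvas while in use.
; Each Tick while Using, DetectHitCanvasActor runs a short forward line trace from the mesh on the BlockAllDynamic profile.
; A hit on a BP_Canvas only prints a debug message; no painting happens here, and the dynamic material creation is unconnected.
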(event `self.ReceiveTick`
  (params (DeltaSeconds :type "Float (single-precision)"))
  (`parent.ReceiveTick` DeltaSeconds)
  ;[1 1 1] If Pickup is using, detect if hit on a canvas
  (if (`self.bUsing`)
    (`self.DetectHitCanvasActor`)))

(fn `DetectHitCanvasActor`
  (bind _mesh (`self.Mesh`))
  (bind _returnvalue (`SceneComponent.K2_GetComponentLocation` _mesh))
  (bind (_outhit _returnvalue_2) (`KismetSystemLibrary.LineTraceSingleByProfile` (+ _returnvalue (0.5 0.0 0.0)) (+ _returnvalue (* (`KismetMathLibrary.GetForwardVector` (`SceneComponent.K2_GetComponentRotation` _mesh)) 15.0)) "BlockAllDynamic"))
  (if _returnvalue_2
    (bind _asbp_canvas (cast `/Game/VRPlayground/Blueprints/PaintCanvas/BP_Canvas` (`.HitActor` (`GameplayStatics.BreakHitResult` _outhit))))
    (`KismetSystemLibrary.PrintString` (`KismetStringLibrary.Concat_StrStr` "HIT TRACE ON: " (`KismetSystemLibrary.GetDisplayName` _asbp_canvas)) true true (struct :`R` 1.0 :`G` 0.101925 :`A` 1.0))))

(fn `UserConstructionScript`
  (`parent.UserConstructionScript`)
  (`|ExecutionSequence`))