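; BP_RopeExample is a VR playground pull-rope example that drops random food pickups through animated trapdoors.
; BeginPlay fills an array of five food pickup Blueprints.
; The OnPull event, raised from C++, runs two timelines that rotate the left and right trapdoors, then spawns a random pickup at SpawnPoint after a brief delay.
; Each pull also plays a duck quack at the world origin.
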(event `self.ReceiveBeginPlay`
  ;[1 1 1] Set Pickup Blueprint Class for selecting a random one
  (set `self.PickupToSpawn` (`|MakeArray` "/Game/VRPlayground/PullingChain/Blueprints/FoodPickups/BP_Fries.BP_Fries_C" "/Game/VRPlayground/PullingChain/Blueprints/FoodPickups/BP_Burger.BP_Burger_C" "/Game/VRPlayground/PullingChain/Blueprints/FoodPickups/BP_Cheese.BP_Cheese_C" "/Game/VRPlayground/PullingChain/Blueprints/FoodPickups/BP_Croissant.BP_Croissant_C" "/Game/VRPlayground/PullingChain/Blueprints/FoodPickups/BP_Chicken.BP_Chicken_C" :!type "Pickup Class Reference")))

(event `self.OnPull`
  (bind _pickuptospawn (`self.PickupToSpawn`))
  ;[1 1 1] Pull Event coming from the C++. Spawn a random actor and play a sound
  (`|ExecutionSequence`
    (:`then_0`
      (`|ExecutionSequence`
        (:`then_0`
          ;[1 1 1] Animate Trapdoors
          (bind (_direction _trapdoorrotation) (`Timeline|TrapdoorLeftTimeline` :!via `PlayFromStart`)
            (:`Update`
              (`SceneComponent.K2_SetWorldRotation` (`self.TrapdoorLeft`) (`KismetMathLibrary.MakeRotator` _trapdoorrotation) false false))))
        (:`then_1`
          (bind (_direction_2 _trapdoorrotation_2) (`Timeline|TimelineRigthTimeline` :!via `PlayFromStart`)
            (:`Update`
              (`SceneComponent.K2_SetWorldRotation` (`self.TrapdooRight`) (`KismetMathLibrary.MakeRotator` _trapdoorrotation_2) false false))))
        (:`then_2`
          (`KismetSystemLibrary.Delay` 0.1)
          ;[1 1 1] Selecting a random Pickup to spawn
          (`|SpawnActorFromClass` (`|GetArrayItem` _pickuptospawn (`KismetMathLibrary.RandomInteger` (`KismetArrayLibrary.Array_Length` _pickuptospawn))) (`KismetMathLibrary.MakeTransform` (`SceneComponent.K2_GetComponentLocation` (`self.SpawnPoint`))) "Undefined" "OverrideRootScale" null null))))
    (:`then_1`
      (`GameplayStatics.PlaySoundAtLocation` "/Game/VRPlayground/Common/Sounds/duck_quack.duck_quack" (0.0 0.0 0.0) (struct) 1.0 1.0 0.0 null null null))))

(fn `UserConstructionScript`)