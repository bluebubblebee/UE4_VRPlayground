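; BP_PaintBrush is a VR paintbrush actor that paints on BP_Canvas actors.
; A short complex line trace from ArrowForward passes the brush, hit mesh and hit result to the canvas's OnPaintVisualTraceLine.
; As a non-VR testing shortcut, Tick traces every frame; the intended Using check is disconnected.
; Debug trace drawing and hit printing remain enabled.
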(event `self.ReceiveTick`
  (params (DeltaSeconds :type "Float (single-precision)"))
  (`parent.ReceiveTick` DeltaSeconds)
  ;[1 0 0.8495] REMOVE THIS AND USE THE BRANCH FOR FINAL VERSION, THIS IS ONLY FOR TESTING WITH NO VR
  (`self.DetectHitCanvasActor`))

(fn `DetectHitCanvasActor`
  (bind _arrowforward (`self.ArrowForward`))
  (bind _returnvalue (`SceneComponent.K2_GetComponentLocation` _arrowforward))
  (bind (_outhit _returnvalue_2) (`KismetSystemLibrary.LineTraceSingleByProfile` :`Start` _returnvalue :`End` (+ _returnvalue (* (`KismetMathLibrary.GetForwardVector` (`SceneComponent.K2_GetComponentRotation` _arrowforward)) 13.0)) :`ProfileName` "BlockAllDynamic" :`bTraceComplex` true :`DrawDebugType` "ForOneFrame"))
  (if _returnvalue_2
    (bind (_bblockinghit _binitialoverlap _time _distance _location _impactpoint _normal _impactnormal _physmat _hitactor _hitcomponent) (`GameplayStatics.BreakHitResult` _outhit))
    (bind _asbp_canvas (cast `/Game/VRPlayground/PaintingCanvas/Blueprints/BP_Canvas` _hitactor))
    (`KismetSystemLibrary.PrintString` (`KismetStringLibrary.Concat_StrStr` "HIT TRACE ON: " (`KismetSystemLibrary.GetDisplayName` _asbp_canvas)) false false (struct :`R` 1.0 :`G` 0.111831 :`A` 1.0) 5.0)
    (bind _asstatic_mesh_component (cast `StaticMeshComponent` _hitcomponent))
    (`KismetSystemLibrary.PrintString` (`KismetSystemLibrary.GetDisplayName` _asstatic_mesh_component) false false (struct :`R` 1.0 :`G` 0.111831 :`A` 1.0) 5.0)
    (`/Game/VRPlayground/PaintingCanvas/Blueprints/BP_Canvas.OnPaintVisualTraceLine` _asbp_canvas self _asstatic_mesh_component _outhit 0.0)))

(fn `UserConstructionScript`
  (`parent.UserConstructionScript`)
  (`|ExecutionSequence`))